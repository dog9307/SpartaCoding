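; Moving actor that oscillates back and forth through its starting location along the Velocity vector.
; BeginPlay stores the start point, and each Tick negates Velocity whenever the distance from that point reaches or exceeds MoveDistance.
; The same Tick then offsets the location by Velocity scaled by delta time, without sweeping for collisions.
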(event `self.ReceiveBeginPlay`
  (set `self.StartPoint` (`self.K2_GetActorLocation`)))

(event `self.ReceiveTick`
  (params (DeltaSeconds :type "Float (single-precision)"))
  (`|ExecutionSequence`
    (:`then_0`
      (if (>= (`KismetMathLibrary.Vector_Distance` (`self.StartPoint`) (`self.K2_GetActorLocation`)) (`self.MoveDistance`))
        (set `self.Velocity` (`KismetMathLibrary.NegateVector` (`self.Velocity`)))))
    (:`then_1`
      (`self.K2_SetActorLocation` (+ (* DeltaSeconds (`self.Velocity`)) (`self.K2_GetActorLocation`))))))

(fn `UserConstructionScript`)