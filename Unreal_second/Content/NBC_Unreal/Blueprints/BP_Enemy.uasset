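; BP_Enemy is an enemy actor with a simple sight system that turns to face the player character while it is in range.
; Begin and end overlap events store or clear a reference to any overlapping BP_Character.
; While that reference is valid, Tick smoothly rotates the actor toward the character by lerping to a look-at rotation with a delta-time-scaled alpha.
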(event `self.ReceiveActorBeginOverlap`
  (params (OtherActor :type "Actor Object Reference"))
  ; 간단한 sight 시스템
  (bind _asbp_character (cast `/Game/NBC_Unreal/Blueprints/BP_Character` OtherActor))
  (set `self.As BP Character` _asbp_character))

(event `self.ReceiveActorEndOverlap`
  (params (OtherActor :type "Actor Object Reference"))
  ; 간단한 sight 시스템
  (cast `/Game/NBC_Unreal/Blueprints/BP_Character` OtherActor)
  (set `self.As BP Character` null))

(event `self.ReceiveTick`
  (params (DeltaSeconds :type "Float (single-precision)"))
  ; 간단한 sight 시스템
  (`/Engine/EditorBlueprintResources/StandardMacros.IsValid` (`self.As BP Character`)
    (:`Is Valid`
      (`self.K2_SetActorRotation` (`KismetMathLibrary.RLerp` (`self.K2_GetActorRotation`) (`KismetMathLibrary.FindLookAtRotation` (`self.K2_GetActorLocation`) (`self.K2_GetActorLocation` (`self.As BP Character`))) (* DeltaSeconds 5.0))))))

(fn `UserConstructionScript`)